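; BP_weapon is a hitscan rifle that can be wielded by the player character, the boss or armed enemies.
; Shoot line-traces from the Barrel socket, applies fixed damage, spends ammo and spawns muzzle, impact and sound effects.
; Reload casts the wielder to play its reload montage, refilling the magazine on completion.
; An empty-magazine event triggers Reload but re-enables CanShoot after a short delay, independently of montage completion.
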(event Custom|out%20of%20ammo?
  ;[1 1 1] out of ammo
  (if (<= (Variables|Default|Getammo) 0)
    (Variables|Default|SetcanShoot? false)
    (CallFunction|Reload)
    (Utilities|FlowControl|Delay 0.2)
    (Variables|Default|SetcanShoot? true)))

(event Custom|Shoot
  (bind _skeletalmesh (Variables|Default|GetSkeletalMesh))
  (bind _skeletalmesh_2 (Variables|Default|GetSkeletalMesh))
  (bind _barrel (Variables|Default|Getbarrel))
  (bind _barrel_2 (Variables|Default|Getbarrel))
  (bind _returnvalue (Transformation|GetSocketTransform _skeletalmesh_2 _barrel_2 "RTS_World"))
  (bind _returnvalue_2 (Transformation|GetSocketTransform _skeletalmesh _barrel "RTS_World"))
  (bind _returnvalue_3 (Math|Vector|GetForwardVector (.rotation _returnvalue_2)))
  (bind _returnvalue_4 (* _returnvalue_3 1e+04))
  ;[1 1 1] SHOOTING
  (Variables|Default|SethitDirection (Math|Vector|Normalize _returnvalue_4))
  (Utilities|Array|AppendArray (Variables|Default|GetActors%20to%20Ignore) (Utilities|Array|MakeArray self))
  (bind _outhit (Collision|LineTraceByChannel (.location _returnvalue_2) (+ (.location _returnvalue_2) _returnvalue_4) "TraceTypeQuery2" true (Variables|Default|GetActors%20to%20Ignore) "None" true "(R=1.000000,G=0.039631,B=0.830314,A=1.000000)"))
  (Variables|Default|SetImpact%20Point (.ImpactPoint (Collision|BreakHitResult _outhit)))
  (Game|Damage|ApplyDamage (.HitActor (Collision|BreakHitResult _outhit)) 5e+01 0 self)
  (Variables|Default|Setammo (- (Variables|Default|Getammo) 1))
  (Effects|SpawnEmitteratLocation "/Game/FPWeapon/effects/M4A1/Effects/MuzzleFlash/P_Muzzle.P_Muzzle" (.location _returnvalue) (.rotation _returnvalue))
  (Audio|PlaySoundatLocation "/Game/FPWeapon/effects/M4A1/Wave/wave_M4A1_shoot.wave_M4A1_shoot" (.location _returnvalue) "0, 0, 0" 1.0 1.0 0.0 0 0 0 0)
  (Effects|SpawnEmitteratLocation "/Game/FPWeapon/effects/M4A1/Effects/MuzzleFlash/P_hit_effect.P_hit_effect" (Variables|Default|GetImpact%20Point) (Math|Conversions|RotationFromXVector (.ImpactNormal (Collision|BreakHitResult _outhit)))))

(event Custom|reload
  (bind _weilder (Variables|Default|GetWeilder))
  ;[1 1 1] reload
  (if (and (< (Variables|Default|Getammo) 30) (not (Variables|Default|GetisReloading?)))
    (Variables|Default|SetcanShoot? false)
    (Variables|Default|SetisReloading? true)
    (Utilities|FlowControl|Sequence
      (:then_0
        (bind _asbp_my_character (Utilities|Casting|CastToBP_myCharacter _weilder))
        (Utilities|IsValid _asbp_my_character
          (:Is%20Valid
            (Animation|Montage|PlayMontage (Variables|/Game/Characters/Blueprints/BP_myCharacter.BP_myCharacter_C|Getfp_mesh _asbp_my_character) "/Game/SK_RifleReload_Montage.SK_RifleReload_Montage"
              (:OnCompleted
                _)))))
      (:then_1
        (bind _asbp_boss (Utilities|Casting|CastToBP_Boss _weilder))
        (Utilities|IsValid _asbp_boss
          (:Is%20Valid
            (Animation|Montage|PlayMontage (Variables|/Script/Engine.Character|GetMesh _asbp_boss) "/Game/Enemy/anim/Reload.Reload"
              (:OnCompleted
                _)))))
      (:then_2
        (bind _asbp_armed_enemy (Utilities|Casting|CastToBP_ArmedEnemy _weilder))
        (Utilities|IsValid _asbp_armed_enemy
          (:Is%20Valid
            (Animation|Montage|PlayMontage (Variables|/Script/Engine.Character|GetMesh _asbp_armed_enemy) "/Game/Enemy/anim/Reload.Reload"
              (:OnCompleted
                _))))))
    (Variables|Default|Setammo 30)
    (Variables|Default|SetisReloading? false)
    (Variables|Default|SetcanShoot? true)))

(fn ConstructionScript)