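; Enemy character Blueprint that senses the player, punches and ragdolls on death.
; Pawn sensing flags the player in the AI blackboard, and Attack plays a punch montage behind a re-entry guard, clearing its blackboard flag on completion.
; Damage from the player lowers health and stores hit data, which aims the impulse on the physics-driven death ragdoll.
; A helper maps Idle, Walk and Run to walk speeds.
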(event OnSeePawn(PawnSensing)
  (params (Pawn :type Pawn%20Object%20Reference))
  ;[1 1 1] on see pawn
  (Utilities|Casting|CastToBP_myCharacter Pawn)
  (AI|Components|Blackboard|SetValueasBool (AI|GetBlackboard (AI|GetAIController self)) (Utilities|Name|MakeLiteralName "hasSeenPlayer?") true))

(event Custom|Attack
  ;[1 1 1] attack
  (if (Variables|Default|GetcanAttack?)
    (Variables|Default|SetcanAttack? false)
    (Animation|Montage|PlayMontage (Variables|Character|GetMesh) "/Game/H2H_PunchCombo01_Montage.H2H_PunchCombo01_Montage"
      (:OnCompleted
        (Pawn|Components|CharacterMovement|SetMovementMode (Variables|Character|GetCharacterMovement) "MOVE_Walking" 0)
        (Variables|Default|SetcanAttack? true)
        (AI|Components|Blackboard|SetValueasBool (AI|GetBlackboard 0) (Utilities|Name|MakeLiteralName "canAttack?") false)))))

(event Custom|ragdoll
  (bind _mesh (Variables|Character|GetMesh))
  ;[1 1 1] rag doll
  (if (Variables|Default|GetisAlive?)
    (Collision|SetCollisionEnabled _mesh "PhysicsOnly")
    (Components|Animation|OverrideAnimationData (Variables|Character|GetMesh) 0 true true 0.0 1.0)
    (Physics|SetSimulatePhysics _mesh true)
    (Class|SkeletalMeshComponent|SetPhysicsBlendWeight _mesh 1.0)
    (Physics|AddImpulseatLocation _mesh (* (Variables|Default|GetHit%20Direction) 2e+03) (Variables|Default|GetImpact%20Point) "None")
    (Variables|Default|SetisAlive? false)
    (Collision|SetCollisionEnabled (Variables|Collision|GetCapsuleComponent) "NoCollision")
    (Collision|SetCollisionResponsetoChannel (Variables|Character|GetMesh) "ECC_Pawn" "ECR_Ignore")))

(event EventBeginPlay)

(event Collision|EventActorBeginOverlap
  (params (OtherActor :type Actor%20Object%20Reference)))

(event EventTick
  (params (DeltaSeconds :type Float%20%28single-precision%29)))

(event Game|Damage|EventAnyDamage
  (params (Damage :type Float%20%28single-precision%29) (DamageType :type Damage%20Type%20Object%20Reference) (InstigatedBy :type Controller%20Object%20Reference) (DamageCauser :type Actor%20Object%20Reference))
  ;[1 1 1] Damage
  (bind _asbp_my_character (Utilities|Casting|CastToBP_myCharacter DamageCauser))
  (Variables|Default|SetHit%20Direction (Variables|/Game/Characters/Blueprints/BP_myCharacter.BP_myCharacter_C|GethitDirection _asbp_my_character))
  (Variables|Default|SetImpact%20Point (Variables|/Game/Characters/Blueprints/BP_myCharacter.BP_myCharacter_C|GetImpact%20Point _asbp_my_character))
  (Variables|Default|SetenemyHealth (- (Variables|Default|GetenemyHealth) Damage))
  (if (<= (Variables|Default|GetenemyHealth) 0.0)
    (CallFunction|Ragdoll)))

(fn ConstructionScript)

(fn SetMovementSpeed
  (params (speed :type E_movementSpeed%20Enum :default "NewEnumerator0"))
  (Variables|/Script/Engine.CharacterMovementComponent|SetMaxWalkSpeed (Variables|Character|GetCharacterMovement) (Utilities|Select :Index speed :NewEnumerator0 0.0 :NewEnumerator1 2e+02 :NewEnumerator2 6e+02))
  (return 0.0))