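; Armed enemy character that fires a hand-socketed BP_weapon, spawned and attached on BeginPlay.
; Pawn sensing sets a blackboard flag on seeing the player, while Attack plays a fire montage to gate shots and SetMovementSpeed maps states to walk speeds.
; Weapon damage lowers health, shown on a camera-facing widget bar.
; At zero health it ragdolls with an impulse along the hit direction and increments the player's kill count.
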(event OnSeePawn(PawnSensing)
  (params (Pawn :type Pawn%20Object%20Reference))
  ;[1 1 1] on see pawn
  (Utilities|Casting|CastToBP_myCharacter Pawn)
  (AI|Components|Blackboard|SetValueasBool (AI|GetBlackboard (AI|GetAIController self)) (Utilities|Name|MakeLiteralName "hasSeenPlayer?") true))

(event Custom|Attack
  (bind _weapon (Variables|Default|Getweapon))
  (bind _weapon_2 (Variables|Default|Getweapon))
  ;[1 1 1] attacking / shooting
  (Default|OutOfAmmo? _weapon)
  (if (and (Variables|Default|GetisAlive?) (Variables|/Game/FPWeapon/blueprints/BP_weapon.BP_weapon_C|GetcanShoot? _weapon))
    (Variables|/Game/FPWeapon/blueprints/BP_weapon.BP_weapon_C|SetcanShoot? _weapon_2 false)
    (Default|Shoot _weapon_2)
    (Utilities|IsValid _weapon_2
      (:Is%20Valid
        (Animation|Montage|PlayMontage (Variables|Character|GetMesh) "/Game/Enemy/anim/Fire_Rifle_Hip_Montage.Fire_Rifle_Hip_Montage"
          (:then
            (Variables|/Game/FPWeapon/blueprints/BP_weapon.BP_weapon_C|SetcanShoot? (Variables|Default|Getweapon) true)))))))

(event Custom|ragdoll
  (bind _mesh (Variables|Character|GetMesh))
  ;[1 1 1] rag doll
  (if (Variables|Default|GetisAlive?)
    (Collision|SetCollisionEnabled _mesh "PhysicsOnly")
    (Components|Animation|OverrideAnimationData (Variables|Character|GetMesh) 0 true true 0.0 1.0)
    (Physics|SetSimulatePhysics _mesh true)
    (Class|SkeletalMeshComponent|SetPhysicsBlendWeight _mesh 1.0)
    (Physics|AddImpulseatLocation _mesh (* (Variables|Default|GetHit%20Direction) 2e+03) (Variables|Default|GetImpact%20Point) "None")
    (Variables|Default|SetisAlive? false)
    (Collision|SetCollisionEnabled (Variables|Collision|GetCapsuleComponent) "NoCollision")
    (Collision|SetCollisionResponsetoChannel (Variables|Character|GetMesh) "ECC_Pawn" "ECR_Ignore")
    (Components|DestroyComponent (Variables|Default|GetHealthBar))))

(event Custom|EquipGun
  ;[1 1 1] add gun to character
  (bind _returnvalue (Game|SpawnActorfromClass "/Game/FPWeapon/blueprints/BP_weapon.BP_weapon_C" (Transformation|GetSocketTransform (Variables|Character|GetMesh) "hand_weapon_r" "RTS_World") "Undefined" "MultiplyWithRoot" 0 0))
  (bind _output_get (Variables|Default|Setweapon _returnvalue))
  (Transformation|AttachComponentToComponent _output_get (Variables|Character|GetMesh) "hand_weapon_r" "SnapToTarget" "SnapToTarget" "KeepRelative" false)
  (bind _returnvalue_2 (Actor|GetActorOfClass "/Game/Enemy/Enemy_BP.Enemy_BP_C"))
  (Utilities|Array|AppendArray (Variables|/Game/FPWeapon/blueprints/BP_weapon.BP_weapon_C|GetActors%20to%20Ignore (Variables|Default|Getweapon)) (Utilities|Array|MakeArray self _returnvalue_2))
  (Variables|/Game/FPWeapon/blueprints/BP_weapon.BP_weapon_C|SetWeilder (Variables|Default|Getweapon) self))

(event EventBeginPlay
  ;[1 1 1] begin play
  (bind _asbp_my_character (Utilities|Casting|CastToBP_myCharacter (Game|GetPlayerCharacter 0)))
  (Variables|Default|SetAs%20BP%20My%20Character _asbp_my_character)
  (CallFunction|EquipGun))

(event Game|Damage|EventAnyDamage
  (params (Damage :type Float%20%28single-precision%29) (DamageType :type Damage%20Type%20Object%20Reference) (InstigatedBy :type Controller%20Object%20Reference) (DamageCauser :type Actor%20Object%20Reference))
  ;[1 1 1] Damage
  (bind _asbp_weapon (Utilities|Casting|CastToBP_weapon DamageCauser))
  (Variables|Default|SetHit%20Direction (Variables|/Game/FPWeapon/blueprints/BP_weapon.BP_weapon_C|GethitDirection _asbp_weapon))
  (Variables|Default|SetImpact%20Point (Variables|/Game/FPWeapon/blueprints/BP_weapon.BP_weapon_C|GetImpact%20Point _asbp_weapon))
  (Variables|Default|SetenemyHealth (- (Variables|Default|GetenemyHealth) Damage))
  (if (<= (Variables|Default|GetenemyHealth) 0.0)
    (CallFunction|Ragdoll)
    (Math|Integer|IncrementInt (Variables|/Game/Characters/Blueprints/BP_myCharacter.BP_myCharacter_C|GetkillCount (Variables|Default|GetAs%20BP%20My%20Character)))))

(event EventTick
  (params (DeltaSeconds :type Float%20%28single-precision%29))
  (bind _healthbar (Variables|Default|GetHealthBar))
  ;[1 1 1] health bar
  (Utilities|IsValid (Variables|Default|GetHealthBar)
    (:Is%20Valid
      (bind _aswb_enemy_health_bar (Utilities|Casting|CastToWB_enemyHealthBar (UserInterface|GetWidget (Variables|Default|GetHealthBar))))
      (Progress|SetPercent (Variables|/Game/Enemy/WB_enemyHealthBar.WB_enemyHealthBar_C|GethealthBar _aswb_enemy_health_bar) (/ (Variables|Default|GetenemyHealth) 1e+02))
      (Transformation|SetWorldRotation _healthbar (Math|Rotator|FindLookatRotation (Transformation|GetWorldLocation _healthbar) (Transformation|GetWorldLocation (Variables|/Script/Engine.PlayerCameraManager|GetTransformComponent (Game|GetPlayerCameraManager 0)))) false false))))

(fn ConstructionScript)

(fn GetRange
  (return 0.0))

(fn SetMovementSpeed
  (params (speed :type E_movementSpeed%20Enum :default "NewEnumerator0"))
  (Variables|/Script/Engine.CharacterMovementComponent|SetMaxWalkSpeed (Variables|Character|GetCharacterMovement) (Utilities|Select :Index speed :NewEnumerator0 0.0 :NewEnumerator1 3e+02 :NewEnumerator2 6e+02 :NewEnumerator3 0.0))
  (return 0.0))